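; BP_Ship is a player-controlled ship that moves along its own forward, right and up vectors through axis-driven movement input.
; Vertical input also snaps the actor's height into a 0 to 500 range before applying movement.
; Left mouse only sets a LeftPressed flag that nothing here reads, and mouse yaw is switched off by a constant branch.
; Control-rotation and camera-arm setup nodes are left unconnected and never run.
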(event `self.ReceiveBeginPlay`)

(event `InputAxis|MoveUp`
  (params (AxisValue :type "Float (single-precision)"))
  (bind _x (.x (`self.K2_GetActorLocation`)))
  (bind _y (.y (`self.K2_GetActorLocation`)))
  (bind _returnvalue (`KismetMathLibrary.FTrunc` (.z (`self.K2_GetActorLocation`))))
  (if (< _returnvalue 500)
    (if (not (> _returnvalue 0))
      (`self.K2_SetActorLocation` (`KismetMathLibrary.MakeVector` _x _y)))
    (else
      (`self.K2_SetActorLocation` (`KismetMathLibrary.MakeVector` _x _y 500.0))))
  (`self.AddMovementInput` (`self.GetActorUpVector`) AxisValue))

(event `InputAxis|MoveRight`
  (params (AxisValue :type "Float (single-precision)"))
  (`self.AddMovementInput` (`self.GetActorRightVector`) AxisValue))

(event `InputAxisKey|MouseX`
  (params (AxisValue :type "Float (single-precision)"))
  (if (not true)
    (`self.AddControllerYawInput` AxisValue)))

(event `Key|LeftMouseButton`
  (params (Key :type "Key Structure"))
  (:`Pressed`
    (set `self.leftPressed` true))
  (:`Released`
    (set `self.leftPressed` false)))

(event `InputAxis|MoveForward`
  (params (AxisValue :type "Float (single-precision)"))
  (`self.AddMovementInput` (`self.GetActorForwardVector`) AxisValue))

(fn `UserConstructionScript`)